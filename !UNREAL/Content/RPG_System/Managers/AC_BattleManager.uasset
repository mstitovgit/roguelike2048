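; Battle manager component for a turn-based RPG that spawns party and enemy actors and tracks whose turn it is.
; Spawn functions resolve Game Instance rosters through data tables, place actors at slot-matched spawn points, and derive each character's targets from enemies assigned to those points.
; ChangeTurn steps through unused slots per side, shows an action widget for characters, and flips sides when exhausted.
; BeginPlay re-caches the Game Instance on a repeating delay.
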(event EventBeginPlay
  ;[1 1 1] Update GI reference
  (bind _asmain_game_instance (Utilities|Casting|CastToMain_GameInstance (Game|GetGameInstance) :!label _label))
  (Variables|Default|SetGameInstanceRef _asmain_game_instance)
  (Utilities|FlowControl|Delay 0.2)
  (goto _label))

(fn SpawnCharacters
  (for _array_element (Variables|/Game/RPG_System/Main_GameInstance.Main_GameInstance_C|GetParty (Variables|Default|GetGameInstanceRef))
    (bind _returnvalue (Utilities|GetDataTableRow "/Game/RPG_System/DataTable/DT_Character.DT_Character" (Utilities|Struct|BreakS_Party _array_element))
      (:then
        (bind _returnvalue_2 (Game|SpawnActorfromClass (.CharacterActorClass (Utilities|Struct|BreakS_Character _returnvalue)) (.TransformLOCAL1 (CallFunction|FindTransform false (.Turn (Utilities|Struct|BreakS_Character _returnvalue)))) "Undefined" 0 self 0 (.Turn (Utilities|Struct|BreakS_Character _returnvalue)) 0))
        (Utilities|Map|Add (Variables|Default|GetSpawnedCharRef) (.Turn (Utilities|Struct|BreakS_Character _returnvalue)) _returnvalue_2)
        (for _array_element_2 (Variables|/Game/RPG_System/SpawnPoints/Character_SpawnPoint.Character_SpawnPoint_C|GetTargetedCharactersBase (.CharacterSpot (CallFunction|FindTransform false (.Turn (Utilities|Struct|BreakS_Character _returnvalue)))))
          (Utilities|Array|Add (Variables|/Game/RPG_System/Managers/AC_CharacterStats.AC_CharacterStats_C|GetTargetedCharacters (Variables|/Game/RPG_System/Character_Base.Character_Base_C|GetAC_CharacterStats _returnvalue_2)) (Variables|/Game/RPG_System/SpawnPoints/Enemy_SpawnPoint.Enemy_SpawnPoint_C|GetAssignedEnemy _array_element_2)))))))

(fn SpawnEnemies
  (bind _gameinstanceref (Variables|Default|GetGameInstanceRef))
  (bind _enemiesononelevel (Variables|/Game/RPG_System/Main_GameInstance.Main_GameInstance_C|GetEnemiesOnOneLevel _gameinstanceref))
  (bind _keys (Utilities|Map|Keys _enemiesononelevel))
  (for _array_element _keys
    (bind _returnvalue (Utilities|GetDataTableRow "/Game/RPG_System/DataTable/DT_Enemies.DT_Enemies" (.Value (Utilities|Map|Find _enemiesononelevel _array_element)))
      (:then
        (bind _returnvalue_2 (Game|SpawnActorfromClass (.EnemyActorClass (Utilities|Struct|BreakS_Enemy _returnvalue)) (.TransformLOCAL1 (CallFunction|FindTransform true (.Turn (Utilities|Struct|BreakS_Enemy _returnvalue)))) "Undefined" 0 self 0 (.Turn (Utilities|Struct|BreakS_Enemy _returnvalue)) 0))
        (Utilities|Map|Add (Variables|Default|GetSpawnedEnemyRef) (.Turn (Utilities|Struct|BreakS_Enemy _returnvalue)) _returnvalue_2)
        (Variables|/Game/RPG_System/SpawnPoints/Enemy_SpawnPoint.Enemy_SpawnPoint_C|SetAssignedEnemy (.EnemySpot (CallFunction|FindTransform true (.Turn (Utilities|Struct|BreakS_Enemy _returnvalue)))) _returnvalue_2)))))

(fn ChangeTurn
  (if (Variables|Default|GetEnemyTurn?)
    (bind _index (Utilities|FlowControl|ForLoopwithBreak 0 3 :!label _label)
      (:LoopBody
        (if (== _index 3)
          (Utilities|Array|Clear (Variables|Default|GetAlreadyUsedCharacters))
          (Variables|Default|Setnextturn 0)
          (Variables|Default|SetCurrentEnemy 0)
          (Variables|Default|SetEnemyTurn? false)
          (else
            (if (.ReturnValue (Utilities|Map|Find (Variables|Default|GetSpawnedEnemyRef) (Variables|Default|Getnextturn)))
              (if (Utilities|Array|ContainsItem (Variables|Default|GetAlreadyUsedCharacters) (.Value (Utilities|Map|Find (Variables|Default|GetSpawnedEnemyRef) (Variables|Default|Getnextturn))))
                _
                (else
                  (bind _output_get (Variables|Default|SetCurrentEnemy (.Value (Utilities|Map|Find (Variables|Default|GetSpawnedEnemyRef) (Variables|Default|Getnextturn)))))
                  (Development|PrintString (Utilities|GetDisplayName _output_get) true true "(R=1.000000,G=0.027705,B=0.000000,A=1.000000)")
                  (Utilities|Array|Add (Variables|Default|GetAlreadyUsedCharacters) _output_get)
                  (goto _label Break))))
            (Variables|Default|Setnextturn (+ (Variables|Default|Getnextturn) 1))))))
    (else
      (CallFunction|RefreshReference)
      (Utilities|IsValid (Variables|Default|GetActionWidget)
        (:Is%20Valid
          (Widget|RemovefromParent (Variables|Default|GetActionWidget)))
        (:Is%20Not%20Valid
          _))
      (bind _index_2 (Utilities|FlowControl|ForLoopwithBreak 0 3 :!label _label_2)
        (:LoopBody
          (if (== _index_2 3)
            (Utilities|Array|Clear (Variables|Default|GetAlreadyUsedCharacters))
            (Variables|Default|Setnextturn 0)
            (Variables|Default|SetCurrentCharacter 0)
            (Variables|Default|SetEnemyTurn? true)
            (Widget|RemovefromParent (Variables|Default|GetActionWidget))
            (elif (.ReturnValue (Utilities|Map|Find (Variables|Default|GetSpawnedCharRef) (Variables|Default|Getnextturn)))
              (if (Utilities|Array|ContainsItem (Variables|Default|GetAlreadyUsedCharacters) (.Value (Utilities|Map|Find (Variables|Default|GetSpawnedCharRef) (Variables|Default|Getnextturn))))
                (Variables|Default|Setnextturn (+ (Variables|Default|Getnextturn) 1) :!label _label_3)
                (else
                  (bind _output_get_2 (Variables|Default|SetCurrentCharacter (.Value (Utilities|Map|Find (Variables|Default|GetSpawnedCharRef) (Variables|Default|Getnextturn)))))
                  (Development|PrintString (Utilities|GetDisplayName _output_get_2))
                  (Utilities|Array|Add (Variables|Default|GetAlreadyUsedCharacters) _output_get_2)
                  (bind _returnvalue (UserInterface|CreateWidget "/Game/RPG_System/UI/WBP_ActionWidget.WBP_ActionWidget_C" (Game|GetPlayerController 0)))
                  (UserInterface|Viewport|AddtoViewport _returnvalue 0)
                  (Variables|Default|SetActionWidget _returnvalue)
                  (Utilities|FlowControl|Sequence
                    (:then_0
                      (goto _label_2 Break))
                    (:then_1
                      ;[1 1 1] debug
                      (for _array_element (Variables|/Game/RPG_System/Managers/AC_CharacterStats.AC_CharacterStats_C|GetTargetedCharacters (Variables|/Game/RPG_System/Character_Base.Character_Base_C|GetAC_CharacterStats _output_get_2))
                        (Development|PrintString (Utilities|GetDisplayName _array_element) true true "(R=1.000000,G=0.000000,B=0.161908,A=1.000000)"))))))
              (else
                (goto _label_3)))))))))

(fn FindTransform
  (params (IsEnemy? :type Boolean) (Turn :type Integer))
  (if IsEnemy?
    (bind _outactors (Actor|GetAllActorsOfClass "/Game/RPG_System/SpawnPoints/Enemy_SpawnPoint.Enemy_SpawnPoint_C"))
    (bind _array_element (Utilities|Array|ForEachLoopwithBreak _outactors :!label _label)
      (:LoopBody
        (if (== (Variables|/Game/RPG_System/SpawnPoints/Enemy_SpawnPoint.Enemy_SpawnPoint_C|Getslotindex _array_element) Turn)
          (LocalVariables|SetTransformLOCAL (Math|Transform|MakeTransform (Transformation|GetActorLocation _array_element) (.rotation (Transformation|GetWorldTransform (Variables|/Game/RPG_System/SpawnPoints/Enemy_SpawnPoint.Enemy_SpawnPoint_C|GetArrow _array_element))) (.scale (Transformation|GetWorldTransform (Variables|/Game/RPG_System/SpawnPoints/Enemy_SpawnPoint.Enemy_SpawnPoint_C|GetArrow _array_element)))))
          (goto _label Break)))
      (:Completed
        (return (LocalVariables|GetTransformLOCAL) _array_element 0)))
    (else
      (bind _outactors_2 (Actor|GetAllActorsOfClass "/Game/RPG_System/SpawnPoints/Character_SpawnPoint.Character_SpawnPoint_C"))
      (bind _array_element_2 (Utilities|Array|ForEachLoopwithBreak _outactors_2 :!label _label_2)
        (:LoopBody
          (if (== (Variables|/Game/RPG_System/SpawnPoints/Character_SpawnPoint.Character_SpawnPoint_C|Getslotindex _array_element_2) Turn)
            (LocalVariables|SetTransformLOCAL (Math|Transform|MakeTransform (Transformation|GetActorLocation _array_element_2) (.rotation (Transformation|GetWorldTransform (Variables|/Game/RPG_System/SpawnPoints/Character_SpawnPoint.Character_SpawnPoint_C|GetArrow _array_element_2))) (.scale (Transformation|GetWorldTransform (Variables|/Game/RPG_System/SpawnPoints/Character_SpawnPoint.Character_SpawnPoint_C|GetArrow _array_element_2)))))
            (goto _label_2 Break)))
        (:Completed
          (return (LocalVariables|GetTransformLOCAL) 0 _array_element_2))))))

(fn RefreshReference
  (bind _values (Utilities|Map|Values (Variables|Default|GetSpawnedCharRef)))
  (for _array_element _values
    (Utilities|Map|Add (Variables|Default|GetSpawnedCharRef) (Variables|/Game/RPG_System/Character_Base.Character_Base_C|GetTurn _array_element) _array_element)))