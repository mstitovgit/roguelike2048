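; AC_CharacterStats is an RPG component that holds a character's stats, display name and current HP.
; SetCharacterData stores those three values as passed in by the caller.
; ReciveDamage subtracts damage from current HP, prints the result as debug output, and calls EventOnDeathMessage on the owner whenever HP is at or below zero.
; HP is not clamped, so further hits after death trigger that call again.
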(fn ReciveDamage
  (params (Damage :type Float%20%28single-precision%29))
  (bind _output_get (Variables|Default|SetCurrentHP (- (Variables|Default|GetCurrentHP) Damage)))
  (Development|PrintString (Utilities|String|ToString(Float) _output_get) true true "(R=0.000000,G=1.000000,B=0.189161,A=1.000000)")
  (if (<= _output_get 0.0)
    (Class|IDamage|EventonDeath(Message) (Components|GetOwner))))

(fn SetCharacterData
  (params (CharacterStats :type Map%20of%20E_CharStats%20Enums%20to%20Float%20%28single-precision%29s :default "NewEnumerator0") (HardDisplayName :type Name) (CurrentHP :type Float%20%28single-precision%29))
  (Variables|Default|SetCharacterStats CharacterStats)
  (Variables|Default|SetHardDisplayName HardDisplayName)
  (Variables|Default|SetCurrentHP CurrentHP))