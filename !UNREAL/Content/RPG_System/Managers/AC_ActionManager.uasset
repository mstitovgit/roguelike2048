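; AC_ActionManager is an RPG component that handles the battle action chosen for the current character.
; SelectAction gets AC_BattleManager from the player controller, stores the action type on the current character's stats component, then switches on it to Attack, Defend or Switch Places handlers.
; The handlers are placeholders: Attack and Defend only print their names, and Switch is empty.
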(event Custom|SelectAction
  (params (ActionType :type E_ActionType%20Enum :default "NewEnumerator0"))
  (bind _output_get (Variables|/Game/RPG_System/Managers/AC_CharacterStats.AC_CharacterStats_C|SetSelectedActionType (Variables|/Game/RPG_System/Character_Base.Character_Base_C|GetAC_CharacterStats (Variables|/Game/RPG_System/Managers/AC_BattleManager.AC_BattleManager_C|GetCurrentCharacter (Actor|GetComponentbyClass (Game|GetPlayerController 0) "/Game/RPG_System/Managers/AC_BattleManager.AC_BattleManager_C"))) ActionType))
  (switch Utilities|FlowControl|Switch|SwitchonE_ActionType _output_get
    (:NewEnumerator1
      (CallFunction|ActivateAttack))
    (:NewEnumerator2
      (CallFunction|ActivateDefend))
    (:NewEnumerator4
      (CallFunction|ActivateSwitch))))

(fn ActivateAttack
  (Development|PrintString "Attack"))

(fn ActivateDefend
  (Development|PrintString "Defend"))

(fn ActivateSwitch)