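; AC_EnemyManager is an RPG battle component that chooses and triggers the current enemy's attack.
; A charged enemy selects targets through the battle manager and uses its special attack; otherwise a random target goes to the game instance before AC_ActionManager and the normal attack run.
; A refresh function fills each spawned enemy's target list from its spawn point's assigned characters.
; BeginPlay caches the game instance in a 0.2-second delay loop.
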(event EventBeginPlay
  (bind _asmain_game_instance (Utilities|Casting|CastToMain_GameInstance (Game|GetGameInstance) :!label _label))
  (Variables|Default|SetGameInstanceRef _asmain_game_instance)
  (Utilities|FlowControl|Delay 0.2)
  (goto _label))

(fn EnemyChooseAttack
  (bind (_currentenemy _battle_manager) (Utilities|CurrentEnemy))
  (if (Variables|/Game/RPG_System/Character_Base.Character_Base_C|GetChargedEnemyAttack _currentenemy)
    (Default|SelectTarget _battle_manager "NewEnumerator3")
    (Default|SpecialAttack _currentenemy)
    (else
      (CallFunction|EnemyChooseTarget))))

(fn EnemyChooseTarget
  (bind _currentenemy (Utilities|CurrentEnemy))
  (Utilities|Array|Add (Variables|/Game/RPG_System/Main_GameInstance.Main_GameInstance_C|GetSelectedCharacterToAction (Variables|Default|GetGameInstanceRef)) (.OutItem (Utilities|Array|Random (Variables|/Game/RPG_System/Managers/AC_CharacterStats.AC_CharacterStats_C|GetTargetedCharacters (Variables|/Game/RPG_System/Character_Base.Character_Base_C|GetAC_CharacterStats _currentenemy)))))
  (Default|ActivateAttack (Actor|GetComponentbyClass (Components|GetOwner) "/Game/RPG_System/Managers/AC_ActionManager.AC_ActionManager_C"))
  (Default|NormalAttack _currentenemy))

(fn RefreshEnemy'sCharVariable
  (bind _outactors (Actor|GetAllActorsOfClass "/Game/RPG_System/SpawnPoints/Enemy_SpawnPoint.Enemy_SpawnPoint_C"))
  (bind _array_element (Utilities|Array|ForEachLoopwithBreak _outactors)
    (:LoopBody
      (Utilities|IsValid (Variables|/Game/RPG_System/SpawnPoints/Enemy_SpawnPoint.Enemy_SpawnPoint_C|GetAssignedEnemy _array_element)
        (:Is%20Valid
          (for _array_element_2 (Variables|/Game/RPG_System/SpawnPoints/Enemy_SpawnPoint.Enemy_SpawnPoint_C|GetAI_TargetedCharactersBase _array_element)
            (Utilities|Array|Add (Variables|/Game/RPG_System/Managers/AC_CharacterStats.AC_CharacterStats_C|GetTargetedCharacters (Variables|/Game/RPG_System/Character_Base.Character_Base_C|GetAC_CharacterStats (Variables|/Game/RPG_System/SpawnPoints/Enemy_SpawnPoint.Enemy_SpawnPoint_C|GetAssignedEnemy _array_element))) (Variables|/Game/RPG_System/SpawnPoints/Character_SpawnPoint.Character_SpawnPoint_C|GetAssignedChar _array_element_2))))))))