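; Inventory actor that stores items as class and amount pairs in a fixed-size slot array, sized at BeginPlay.
; AddItem tops up a matching stack or takes an empty slot, calling itself recursively for overflow up to MaxStackSize and for each unstackable unit.
; Search helpers locate slots, GetItemInfo reads item data from class defaults, and DeleteItem clears a slot by index.
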(event EventBeginPlay
  (Utilities|Array|Resize (Variables|Default|GetSlots) (Variables|Default|GetSlotsAmount)))

(event Collision|EventActorBeginOverlap
  (params (OtherActor :type Actor%20Object%20Reference)))

(event EventTick
  (params (DeltaSeconds :type Float%20%28single-precision%29)))

(fn ConstructionScript)

(fn IsSlotEmpty
  (params (SlotIndex :type Integer))
  (return (not (Utilities|IsValidClass (.itemclass (Utilities|Array|Get(acopy) (Variables|Default|GetSlots) SlotIndex))))))

(fn AddItem
  (params (ItemClass :type Item%20Master%20Class%20Reference) (Amount :type Integer))
  (LocalVariables|SetLocalAmount Amount)
  (LocalVariables|SetLocalItemClass ItemClass)
  (if (.CanBeStacked (Utilities|Struct|BreakItemStructure (Utilities|GetClassDefaults ItemClass)))
    (bind (_success _index) (CallFunction|SearchFreeStack (LocalVariables|GetLocalItemClass)))
    (if _success
      (bind _output_get (LocalVariables|SetLocalFoundIndex _index))
      (if (> (+ (.amount (Utilities|Array|Get(acopy) (Variables|Default|GetSlots) _output_get)) (LocalVariables|GetLocalAmount)) (Variables|Default|GetMaxStackSize))
        (Utilities|Array|SetArrayElem (Variables|Default|GetSlots) (LocalVariables|GetLocalFoundIndex) (Utilities|Struct|MakeSlotStructure (LocalVariables|GetLocalItemClass) (Variables|Default|GetMaxStackSize)))
        (CallFunction|AddItem (LocalVariables|GetLocalItemClass) (- (+ (.amount (Utilities|Array|Get(acopy) (Variables|Default|GetSlots) _output_get)) (LocalVariables|GetLocalAmount)) (LocalVariables|GetLocalAmount)))
        (return true)
        (else
          (Utilities|Array|SetArrayElem (Variables|Default|GetSlots) (LocalVariables|GetLocalFoundIndex) (Utilities|Struct|MakeSlotStructure (LocalVariables|GetLocalItemClass) (+ (.amount (Utilities|Array|Get(acopy) (Variables|Default|GetSlots) _output_get)) (LocalVariables|GetLocalAmount))))
          (return true)))
      (else
        (bind (_success_2 _index_2) (CallFunction|SearchEmptySlot))
        (if _success_2
          (LocalVariables|SetLocalFoundIndex _index_2)
          (if (> (LocalVariables|GetLocalAmount) (Variables|Default|GetMaxStackSize))
            (Utilities|Array|SetArrayElem (Variables|Default|GetSlots) (LocalVariables|GetLocalFoundIndex) (Utilities|Struct|MakeSlotStructure (LocalVariables|GetLocalItemClass) (Variables|Default|GetMaxStackSize)))
            (CallFunction|AddItem (LocalVariables|GetLocalItemClass) (- (LocalVariables|GetLocalAmount) (Variables|Default|GetMaxStackSize)))
            (return true)
            (else
              (Utilities|Array|SetArrayElem (Variables|Default|GetSlots) (LocalVariables|GetLocalFoundIndex) (Utilities|Struct|MakeSlotStructure (LocalVariables|GetLocalItemClass) (LocalVariables|GetLocalAmount)))
              (return true)))
          (else
            (return false)))))
    (else
      (bind (_success_3 _index_3) (CallFunction|SearchEmptySlot))
      (if _success_3
        (Utilities|Array|SetArrayElem (Variables|Default|GetSlots) _index_3 (Utilities|Struct|MakeSlotStructure (LocalVariables|GetLocalItemClass) 1))
        (if (> (LocalVariables|GetLocalAmount) 1)
          (CallFunction|AddItem (LocalVariables|GetLocalItemClass) (- (LocalVariables|GetLocalAmount) 1)))
        (return true)
        (else
          (return false))))))

(fn GetItemInfo
  (params (index :type Integer))
  (bind _slots (Variables|Default|GetSlots))
  (bind _output (Utilities|Array|Get(acopy) _slots index))
  (if (Utilities|IsValidClass (.itemclass _output))
    (return (Utilities|GetClassDefaults (.itemclass _output)) (.itemclass _output) (.amount _output) false)
    (else
      (return "" 0 0 true))))

(fn SearchEmptySlot
  (bind _array_index (Utilities|Array|ForEachLoopwithBreak (Variables|Default|GetSlots) :!label _label)
    (:LoopBody
      (bind _empty (CallFunction|IsSlotEmpty _array_index))
      (if _empty
        (LocalVariables|SetLocalIndex _array_index)
        (LocalVariables|SetLocalSuccess true)
        (goto _label Break)))
    (:Completed
      (return (LocalVariables|GetLocalSuccess) (LocalVariables|GetLocalIndex)))))

(fn SearchFreeStack
  (params (ItemClass :type Item%20Master%20Class%20Reference))
  (bind (_array_element _array_index) (Utilities|Array|ForEachLoopwithBreak (Variables|Default|GetSlots) :!label _label)
    (:LoopBody
      (if (Utilities|IsValidClass (.ItemClass (Utilities|Struct|BreakSlotStructure _array_element)))
        (if (and (== (.ItemClass (Utilities|Struct|BreakSlotStructure _array_element)) ItemClass) (< (.Amount (Utilities|Struct|BreakSlotStructure _array_element)) (Variables|Default|GetMaxStackSize)))
          (LocalVariables|SetLocalBool true)
          (LocalVariables|SetLocalIndex _array_index)
          (goto _label Break))))
    (:Completed
      (return (LocalVariables|GetLocalBool) (LocalVariables|GetLocalIndex)))))

(fn DeleteItem
  (params (index :type Integer))
  (bind _slots (Variables|Default|GetSlots))
  (Utilities|Array|SetArrayElem _slots index (Utilities|Struct|MakeSlotStructure))
  (Development|PrintString (Utilities|GetClassDisplayName (.ItemClass (Utilities|Struct|BreakSlotStructure (Utilities|Array|Get(acopy) _slots index))))))