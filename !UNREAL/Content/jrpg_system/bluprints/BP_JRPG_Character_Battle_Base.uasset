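; Base character Blueprint for JRPG battles, providing mouse targeting and stub hooks for combat.
; While targeting is enabled, hovering the capsule shows or hides targets through the targeting manager.
; Clicking a character that is among the targeted ones asks the battle manager to execute the action on all targeted characters.
; Damage, death, heal, resurrection and action events are empty, and state getters return fixed defaults, apparently for child classes to override.
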(event OnBeginCursorOver(CapsuleComponent)
  (params (TouchedComponent :type Primitive%20Component%20Object%20Reference))
  ;[1 1 1] show target point over character head
  (bind _targetingmanagerref (Variables|Default|GetTargetingManagerRef)
    (:then
      (if (Variables|/Game/jrpg_system/bluprints/Components/AC_TargetingManager.AC_TargetingManager_C|GetTargetingEnabled? _targetingmanagerref)
        (Default|ShowTargets _targetingmanagerref)))
    (:else)))

(event OnEndCursorOver(CapsuleComponent)
  (params (TouchedComponent :type Primitive%20Component%20Object%20Reference))
  ;[1 1 1] show target point over character head
  (bind _targetingmanagerref (Variables|Default|GetTargetingManagerRef)
    (:then
      (if (Variables|/Game/jrpg_system/bluprints/Components/AC_TargetingManager.AC_TargetingManager_C|GetTargetingEnabled? _targetingmanagerref)
        (Default|HideTargets _targetingmanagerref)))
    (:else)))

(event OnClicked(CapsuleComponent)
  (params (TouchedComponent :type Primitive%20Component%20Object%20Reference) (ButtonPressed :type Key%20Structure :default "None"))
  ;[1 1 1] character will execute selected action
  (bind _targetingmanagerref (Variables|Default|GetTargetingManagerRef)
    (:then
      (if (Variables|/Game/jrpg_system/bluprints/Components/AC_TargetingManager.AC_TargetingManager_C|GetTargetingEnabled? _targetingmanagerref)
        (if (Utilities|Array|ContainsItem (Variables|/Game/jrpg_system/bluprints/Components/AC_TargetingManager.AC_TargetingManager_C|GetTargetedCharacters _targetingmanagerref) self)
          (bind _battlemanager (Variables|Default|GetBattleManager)
            (:then
              (Default|RequestActionExecution _battlemanager (Variables|/Game/jrpg_system/bluprints/Components/AC_TargetingManager.AC_TargetingManager_C|GetTargetedCharacters _targetingmanagerref)))
            (:else)))))
    (:else)))

(event EventOnDamageRecived
  (params (Damage :type Float%20%28single-precision%29) (Critical? :type Boolean)))

(event EventOnDeath)

(event EventOnHealed
  (params (RestoredMP? :type Boolean) (HealAmount :type Float%20%28single-precision%29)))

(event EventOnRessurected
  (params (HealAmount :type Float%20%28single-precision%29)))

(event Custom|ExecuteAction)

(fn ConstructionScript)

(fn ApplyAttackEffect)

(fn GetCharacterCombatClass
  (return "NewEnumerator0"))

(fn GetIsDead
  (return false))

(fn GetIsDefending
  (return false))