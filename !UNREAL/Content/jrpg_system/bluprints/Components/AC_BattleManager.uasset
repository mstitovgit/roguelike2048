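; Battle manager component for a JRPG turn-based combat system, built around initiative-based turn order.
; BeginPlay caches the custom GameInstance, retrying after a short delay until the cast succeeds.
; ResumeBattle triggers a delayed turn check while both sides have members, searching for a full initiative bar with player characters prioritized over enemies.
; Initiative increments, use of the search result, battle end, game over and action execution are not implemented here.
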(event EventBeginPlay
  (bind _asgi_custom (Utilities|Casting|CastToGI_Custom (Game|GetGameInstance) :!label _label)
    (:then
      (Variables|Default|SetGameInstanceReference _asgi_custom))
    (:CastFailed
      (Utilities|FlowControl|Delay 0.2)
      (goto _label))))

(event Custom|ResumeBattle
  (CallFunction|AddInitiativetoAllCharacters))

(event Custom|AddInitiativeToAllCharacters
  (Utilities|FlowControl|Delay 0.2)
  (if (Math|Boolean|NORBoolean (== (Utilities|Array|Length (Variables|BattleInProgress|GetPlayerCharacters)) 0) (== (Utilities|Array|Length (Variables|BattleInProgress|GetEnemies)) 0)) ; Battle cannot be continued if \nall player characters or enemies are dead.
    (CallFunction|GetCharacterwithMaxInitiative)))

(event Custom|EndBattle)

(event Custom|GameOver)

(fn GetCharacterwithMaxInitiative
  ;[1 1 1] Check if there is player character with full initiative bar.
  (for _array_element (Variables|BattleInProgress|GetPlayerCharacters)
    (if (>= (Variables|/Game/jrpg_system/bluprints/Components/AC_Character_BattleStats.AC_Character_BattleStats_C|GetCurrenInitiative (Variables|/Game/jrpg_system/bluprints/BP_JRPG_Character_Battle_Base.BP_JRPG_Character_Battle_Base_C|GetCharacter_BattleStats _array_element)) (Variables|Default|GetInitiativeNeededToTakePlace))
      (LocalVariables|SetSucsess?LOCAL true)
      (LocalVariables|SetCharacterLOCAL _array_element)))
  (if (LocalVariables|GetSucsess?LOCAL) ; If player character was found it will be his turn.
    (return (LocalVariables|GetSucsess?LOCAL) (LocalVariables|GetCharacterLOCAL))
    (else
      ;[1 1 1] If there is no player character with full initiative check if there is enemy with full initiation bar.
      (for _array_element_2 (Variables|BattleInProgress|GetEnemies)
        (if (>= (Variables|/Game/jrpg_system/bluprints/Components/AC_Character_BattleStats.AC_Character_BattleStats_C|GetCurrenInitiative (Variables|/Game/jrpg_system/bluprints/BP_JRPG_Character_Battle_Base.BP_JRPG_Character_Battle_Base_C|GetCharacter_BattleStats _array_element_2)) (Variables|Default|GetInitiativeNeededToTakePlace))
          (LocalVariables|SetSucsess?LOCAL true)
          (LocalVariables|SetCharacterLOCAL _array_element_2)))
      (return (LocalVariables|GetSucsess?LOCAL) (LocalVariables|GetCharacterLOCAL)))))

(fn RequestActionExecution
  (params (TargetedCharacters :type Array%20of%20BP%20JRPG%20Character%20Battle%20Base%20Object%20References))
  ;[1 1 1] executing char action/animation in main BP
)