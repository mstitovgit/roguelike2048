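; Actor component for the JRPG system that tracks targeting state: whether targeting is enabled, whether self-targeting is allowed, and which targeting type is selected.
; BeginPlay caches the custom game instance, retrying the cast after a short delay until it succeeds.
; Enable, Disable and Cancel functions set the state.
; ShowTargets and HideTargets are unfinished: the former stores the indicated character and switches on type without further logic, the latter is empty.
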(event EventBeginPlay
  (bind _asgi_custom (Utilities|Casting|CastToGI_Custom (Game|GetGameInstance) :!label _label)
    (:then
      (Variables|Default|SetGameInstanceRef _asgi_custom))
    (:CastFailed
      (Utilities|FlowControl|Delay 0.2)
      (goto _label))))

(fn ShowTargets
  (params (IndicatedCharacterLOCAL1 :type BP%20JRPG%20Character%20Battle%20Base%20Object%20Reference))
  (LocalVariables|SetIndicatedCharacterLOCAL IndicatedCharacterLOCAL1)
  (switch Utilities|FlowControl|Switch|SwitchonE_TargetingType (Variables|Default|GetSelectTargetingType)))

(fn HideTargets)

(fn EnableTargeting
  (params (CanTargetSelf? :type Boolean) (SelectTargetingType :type E_TargetingType%20Enum :default "NewEnumerator0"))
  (Variables|Default|SetCanTargetSelf? CanTargetSelf?)
  (Variables|Default|SetSelectTargetingType SelectTargetingType)
  (Variables|Default|SetTargetingEnabled? true))

(fn DisableTargeting
  (Variables|Default|SetTargetingEnabled? false))

(fn CancelTargeting
  (if (Variables|Default|GetTargetingEnabled?)
    (Variables|Default|SetTargetingEnabled? false)))